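; Block is a shootable minesweeper-style grid block that has a one-in-five chance of containing a mine, rolled at BeginPlay.
; Its hit event, re-bound every Tick, responds only to first-person projectiles, destroying both projectile and block.
; It reports to the level's MineGrid as either a detonated mine or a removed block.
; Mined blocks also spawn an explosion effect at their X/Y and a fixed height.
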(event Custom|OnActorHit_Event
  (params (SelfActor :type Actor%20Object%20Reference) (OtherActor :type Actor%20Object%20Reference) (NormalImpulse :type Vector) (Hit :type Hit%20Result%20Structure%20%28by%20ref%29))
  (bind _returnvalue (Transformation|GetActorLocation))
  (bind _reference_to_minegrid (Variables|Default|GetReference%20to%20MineGrid))
  (bind (_x _y) (Math|Vector|BreakVector _returnvalue))
  (if (Utilities|ClassIsChildOf (Utilities|GetClass OtherActor) "/Game/FirstPerson/Blueprints/BP_FirstPersonProjectile.BP_FirstPersonProjectile_C")
    (Actor|DestroyActor OtherActor)
    (if (Variables|Default|GetContainsMine)
      (Default|DetonatedMine _reference_to_minegrid)
      (Game|SpawnActorfromClass "/Game/StarterContent/Blueprints/Blueprint_Effect_Explosion.Blueprint_Effect_Explosion_C" (Math|Transform|MakeTransform (Math|Vector|MakeVector _x _y -5.5e+02)) "AlwaysSpawn" "MultiplyWithRoot" 0 0)
      (Actor|DestroyActor)
      (else
        (Default|RemovedBlock _reference_to_minegrid)
        (Actor|DestroyActor)))))

(event EventBeginPlay
  (bind _returnvalue (Actor|GetActorOfClass "/Game/Blueprints/MineGrid.MineGrid_C"))
  (Variables|Default|SetReference%20to%20MineGrid _returnvalue)
  (if (Math|Conversions|ToBoolean(Integer) (Math|Random|RandomInteger 5))
    (Variables|Default|SetContainsMine false)
    (else
      (Variables|Default|SetContainsMine true))))

(event Collision|EventActorBeginOverlap
  (params (OtherActor :type Actor%20Object%20Reference)))

(event EventTick
  (params (DeltaSeconds :type Float%20%28single-precision%29))
  (Collision|BindEventtoOnActorHit (delegate Custom|OnActorHit_Event)))

(fn ConstructionScript)