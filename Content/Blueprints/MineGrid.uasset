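; MineGrid spawns and tracks the Block grid for a Minesweeper-style game.
; On BeginPlay it lays out blocks in evenly spaced rows and columns, tallying blocks and those containing mines.
; A second pass runs a sphere overlap at each block to fill its NearbyMines count.
; DetonatedMine and RemovedBlock update the remaining mine, detonation and block counters.
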(event EventBeginPlay
  ;[1 1 1] Create the grid of blocks
  (for _index (range 0 10)
    (for _index_2 (range 0 10)
      (bind _returnvalue (Game|SpawnActorfromClass "/Game/Blueprints/Block.Block_C" (Math|Transform|MakeTransform (Math|Vector|MakeVector (Math|Conversions|ToFloat(Integer) (* _index_2 300)) (Math|Conversions|ToFloat(Integer) (* _index 300)) 0.0)) "AdjustIfPossibleButAlwaysSpawn" "MultiplyWithRoot" 0 0))
      (Variables|Default|SetNumBlocks (+ (Variables|Default|GetNumBlocks) 1))
      (if (Variables|/Game/Blueprints/Block.Block_C|GetContainsMine _returnvalue)
        (Variables|Default|SetNumMines (+ (Variables|Default|GetNumMines) 1)))))
  ;[1 1 1] Initializes value to contain the number of nearby mines at each block
  (bind _outactors (Actor|GetAllActorsOfClass "/Game/Blueprints/Block.Block_C"))
  (for _array_element _outactors
    (bind _outactors_2 (Collision|SphereOverlapActors (Transformation|GetActorLocation _array_element) 5e+02 (Utilities|Array|MakeArray "ObjectTypeQuery1") "/Game/Blueprints/Block.Block_C"))
    (for _array_element_2 _outactors_2
      (bind _asblock (Utilities|Casting|CastToBlock _array_element_2))
      (if (Variables|/Game/Blueprints/Block.Block_C|GetContainsMine _asblock)
        (Math|Integer|IncrementInt (Variables|/Game/Blueprints/Block.Block_C|GetNearbyMines _array_element))))))

(event Collision|EventActorBeginOverlap
  (params (OtherActor :type Actor%20Object%20Reference)))

(fn ConstructionScript)

(fn DetonatedMine
  (Variables|Default|SetNumMines (- (Variables|Default|GetNumMines) 1))
  (Variables|Default|SetNumDetonated (+ (Variables|Default|GetNumDetonated) 1))
  (CallFunction|RemovedBlock))

(fn RemovedBlock
  (Variables|Default|SetNumBlocks (- (Variables|Default|GetNumBlocks) 1)))